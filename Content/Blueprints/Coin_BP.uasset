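; Coin actor that spins and bobs in place; its overlap event is empty, so no pickup logic lives in this graph.
; BeginPlay caches the spawn location as the anchor for the motion.
; Each Tick applies frame-rate-independent yaw rotation and sets height from a degree-based sine of game time, with tunable rotation speed, bob speed and offset, keeping X and Y fixed.
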(event `self.ReceiveActorBeginOverlap`
  (params (OtherActor :type "Actor Object Reference")))

(event `self.ReceiveBeginPlay`
  (bind (_returnvalue_x _returnvalue_y _returnvalue_z) (`KismetMathLibrary.BreakVector` (`self.K2_GetActorLocation`)))
  (set `self.initialX` _returnvalue_x)
  (set `self.initialY` _returnvalue_y)
  (set `self.intialZ` _returnvalue_z))

(event `self.ReceiveTick`
  (params (DeltaSeconds :type "Float (single-precision)"))
  (`self.K2_AddActorLocalRotation` (`KismetMathLibrary.MakeRotator` 0.0 0.0 (* (`self.rotationSpeed`) (`GameplayStatics.GetWorldDeltaSeconds`))))
  (bind _output_get (set `self.newZ` (+ (`self.intialZ`) (* (`KismetMathLibrary.DegSin` (* (`GameplayStatics.GetTimeSeconds`) (`self.upAndDownSpeed`))) (`self.upAndDownOffset`)))))
  (`self.K2_SetActorLocation` (`KismetMathLibrary.MakeVector` (`self.initialX`) (`self.initialY`) _output_get)))

(fn `UserConstructionScript`)